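; Endless-runner tunnel segment with a rotating holed wall, a possible health pack and an enemy.
; Randomize functions, not called here, vary the wall mesh and roll, and pickup and enemy placement.
; The end trigger spawns the next tunnel via TunnelSpawner, destroys this one, and rewards unbonked passes with score and speed.
; Walls and enemies damage BP_Player, prompting restart at zero health; shooting enemies adds score but reduces speed.
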(event `self.ReceiveBeginPlay`
  (bind _asbp_player (cast `/Game/InfiniteMatrix/Blueprints/BP_Player` (`GameplayStatics.GetPlayerPawn` 0)))
  (set `self.Player` _asbp_player))

(event `self.ReceiveTick`
  (params (DeltaSeconds :type "Float (single-precision)"))
  (`SceneComponent.K2_AddLocalRotation` (`self.WallMesh`) (`KismetMathLibrary.MakeRotator` (* DeltaSeconds (`self.RotateSpeed`))) false false))

(event `self.TriggerZone.OnComponentBeginOverlap`
  (params (OverlappedComponent :type "PrimitiveComponent Object Reference") (OtherActor :type "Actor Object Reference") (OtherComp :type "PrimitiveComponent Object Reference") (OtherBodyIndex :type Integer) (bFromSweep :type Boolean) (SweepResult :type "HitResult Structure (by ref)"))
  (bind _player (`self.Player`))
  (bind _player_2 (`self.Player`))
  (cast `/Game/InfiniteMatrix/Blueprints/BP_Player` OtherActor)
  (`/Game/InfiniteMatrix/Blueprints/BP_TunnelSpawner.Spawn Tunnel at Spawn Pt` (`self.TunnelSpawner`))
  (`self.K2_DestroyActor`)
  (if (`self.Bonked`)
    (set `self.Bonked` false)
    (else
      (set `/Game/InfiniteMatrix/Blueprints/BP_Player.Score` (+ (`/Game/InfiniteMatrix/Blueprints/BP_Player.Score` _player_2) 1) _player_2)
      (set `/Game/InfiniteMatrix/Blueprints/BP_Player.ForwardSpeed` (+ (`/Game/InfiniteMatrix/Blueprints/BP_Player.ForwardSpeed` _player) 50.0) _player))))

(event `self.WallMesh.OnComponentBeginOverlap`
  (params (OverlappedComponent :type "PrimitiveComponent Object Reference") (OtherActor :type "Actor Object Reference") (OtherComp :type "PrimitiveComponent Object Reference") (OtherBodyIndex :type Integer) (bFromSweep :type Boolean) (SweepResult :type "HitResult Structure (by ref)"))
  (`|ExecutionSequence`
    (:`then_0`
      (bind _asbp_player (cast `/Game/InfiniteMatrix/Blueprints/BP_Player` OtherActor))
      (bind _output_get (set `/Game/InfiniteMatrix/Blueprints/BP_Player.Health` (- (`/Game/InfiniteMatrix/Blueprints/BP_Player.Health` _asbp_player) 1) _asbp_player))
      (set `self.Bonked` true)
      (if (== _output_get 0)
        (`/Game/InfiniteMatrix/Blueprints/BP_Player.DisplayRestart` _asbp_player)))
    (:`then_1`
      (bind _asbp_projectile (cast `/Game/InfiniteMatrix/Blueprints/BP_Projectile` OtherActor))
      (`self.K2_DestroyActor` _asbp_projectile))))

(event `self.Health Pack.OnComponentHit`
  (params (HitComponent :type "PrimitiveComponent Object Reference") (OtherActor :type "Actor Object Reference") (OtherComp :type "PrimitiveComponent Object Reference") (NormalImpulse :type "Vector Structure") (Hit :type "HitResult Structure (by ref)"))
  (bind _asbp_player (cast `/Game/InfiniteMatrix/Blueprints/BP_Player` OtherActor))
  (set `/Game/InfiniteMatrix/Blueprints/BP_Player.Health` (`KismetMathLibrary.Min` (+ (`/Game/InfiniteMatrix/Blueprints/BP_Player.Health` _asbp_player) 1) 4) _asbp_player)
  (`ActorComponent.K2_DestroyComponent` (`self.Health Pack`)))

(event `self.Enemy #1.OnComponentHit`
  (params (HitComponent :type "PrimitiveComponent Object Reference") (OtherActor :type "Actor Object Reference") (OtherComp :type "PrimitiveComponent Object Reference") (NormalImpulse :type "Vector Structure") (Hit :type "HitResult Structure (by ref)"))
  (bind _player (`self.Player`))
  (bind _player_2 (`self.Player`))
  (bind _player_3 (`self.Player`))
  (cast `/Game/InfiniteMatrix/Blueprints/BP_Player` OtherActor
    (:`then`
      (`ActorComponent.K2_DestroyComponent` (`self.Enemy #1`))
      (bind _output_get (set `/Game/InfiniteMatrix/Blueprints/BP_Player.Health` (- (`/Game/InfiniteMatrix/Blueprints/BP_Player.Health` _player_2) 1) _player_2))
      (if (<= _output_get 0)
        (`/Game/InfiniteMatrix/Blueprints/BP_Player.DisplayRestart` _player_2)))
    (:`CastFailed`
      (cast `/Game/InfiniteMatrix/Blueprints/BP_Projectile` OtherActor)
      (`ActorComponent.K2_DestroyComponent` (`self.Enemy #1`))
      (set `/Game/InfiniteMatrix/Blueprints/BP_Player.Score` (+ (`/Game/InfiniteMatrix/Blueprints/BP_Player.Score` _player) 1) _player)
      (set `/Game/InfiniteMatrix/Blueprints/BP_Player.ForwardSpeed` (- (`/Game/InfiniteMatrix/Blueprints/BP_Player.ForwardSpeed` _player_3) 25.0) _player_3))))

(fn `RandomizePills`
  (bind _health_pack (`self.Health Pack`))
  (bind _enemy__1 (`self.Enemy #1`))
  (`|ExecutionSequence`
    (:`then_0`
      (if (> (`KismetMathLibrary.RandomIntegerInRange` 1 100) 75)
        (`SceneComponent.K2_AddLocalOffset` _health_pack (`KismetMathLibrary.MakeVector` (`KismetMathLibrary.RandomFloatInRange` 800.0 2000.0) (`KismetMathLibrary.RandomFloatInRange` -1270.0 -730.0) (`KismetMathLibrary.RandomFloatInRange` -270.0 270.0)) false false)
        (`SceneComponent.K2_AddLocalRotation` (`self.Health Pack`) (`KismetMathLibrary.MakeRotator` (`KismetMathLibrary.RandomFloatInRange` 0.0 360.0) (`KismetMathLibrary.RandomFloatInRange` 0.0 360.0)) false false)
        (else
          (`ActorComponent.K2_DestroyComponent` _health_pack))))
    (:`then_1`
      (`SceneComponent.K2_AddLocalOffset` _enemy__1 (`KismetMathLibrary.MakeVector` (`KismetMathLibrary.RandomFloatInRange` 800.0 2300.0) (`KismetMathLibrary.RandomFloatInRange` -270.0 270.0) (`KismetMathLibrary.RandomFloatInRange` -270.0 270.0)) false false)
      (`SceneComponent.K2_AddLocalRotation` _enemy__1 (`KismetMathLibrary.MakeRotator` (`KismetMathLibrary.RandomFloatInRange` 0.0 360.0) (`KismetMathLibrary.RandomFloatInRange` 0.0 360.0)) false false))))

(fn `RandomizeWalls`
  (`StaticMeshComponent.SetStaticMesh` (`self.WallMesh`) (select `int` (`KismetMathLibrary.RandomIntegerInRange` 0 3) :`0` "/Game/InfiniteMatrix/Meshes/SM_Hole_01.SM_Hole_01" :`1` "/Game/InfiniteMatrix/Meshes/SM_Hole_02.SM_Hole_02" :`2` "/Game/InfiniteMatrix/Meshes/SM_Hole_03.SM_Hole_03" :`3` "/Game/InfiniteMatrix/Meshes/SM_Hole_04.SM_Hole_04" :!type "StaticMesh Object Reference"))
  (`SceneComponent.K2_AddLocalRotation` (`self.WallMesh`) (`KismetMathLibrary.MakeRotator` (`KismetMathLibrary.RandomFloatInRange` 0.0 360.0)) false false))

(fn `UserConstructionScript`)